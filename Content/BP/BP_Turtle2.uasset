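; BP_Turtle2 is a turtle actor that moves forward in a stop-and-go rhythm.
; Its MoveTurtle event takes a delta time and uses a Wait flag and an accumulating timer to alternate about a second of movement with a half-second pause.
; Movement is delegated to MoveForward, which is not defined in this Blueprint, and Tick is unused.
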(event EventBeginPlay
  (Variables|Default|SetWait false)
  (Variables|Default|SetTimer 0.0))

(event Collision|EventActorBeginOverlap
  (params (OtherActor :type Actor%20Object%20Reference)))

(event EventTick
  (params (DeltaSeconds :type Float%20%28single-precision%29)))

(event EventMoveTurtle
  (params (DeltaTime :type Float%20%28single-precision%29))
  (if (Variables|Default|GetWait)
    (bind _output_get (Variables|Default|SetTimer (+ (Variables|Default|GetTimer) DeltaTime)))
    (if (> _output_get 0.5)
      (Variables|Default|SetWait false)
      (Variables|Default|SetTimer 0.0))
    (else
      (bind _output_get_2 (Variables|Default|SetTimer (+ (Variables|Default|GetTimer) DeltaTime)))
      (Class|Turtle|MoveForward DeltaTime)
      (if (> _output_get_2 1.0)
        (Variables|Default|SetWait true)
        (Variables|Default|SetTimer 0.0)))))

(fn ConstructionScript)